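; BP_RenderBase is the mini-game render actor that holds the game root, an info widget, a background image, and occlusion and fade spheres.
; Dynamic materials created for the two spheres expose occlusion color and fade opacity as parameters.
; Events forward completion counts, timer, visibility and help text to the widget through interface messages.
; Other events offset the game root and UI for VR and toggle the background image.
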(event Custom|CreateDynamicMaterial
  ;[1 1 1] Create dynamic materials for occlusion sphere and fade sphere
  (bind _returnvalue (Rendering|Material|CreateDynamicMaterialInstance (Variables|Default|GetSM_OcclusionSphere) 0 "/Game/MiniGames/Materials/M_OcclusionBackground.M_OcclusionBackground" :!class /Script/Engine.PrimitiveComponent))
  (Variables|Default|SetOcclusionSphereMaterialInst _returnvalue)
  (bind _returnvalue_2 (Rendering|Material|CreateDynamicMaterialInstance (Variables|Default|GetSM_FadeSphere) 0 "/Game/MiniGames/Materials/M_FadeSphere.M_FadeSphere" :!class /Script/Engine.PrimitiveComponent))
  (Variables|Default|SetFadeSphereMaterialInst _returnvalue_2))

(event Custom|SetInfoValues
  (params (CompleteCurrent :type Integer) (CompleteMax :type Integer) (Timer :type Float%20%28single-precision%29))
  ;[1 1 1] Pass UI values - Complete current, Max complete, Timer to UI widget. Use Interface
  (Class|IMiniGameWidgetInteface|SetWidgetValues(Message) (UserInterface|GetUserWidgetObject (Variables|Default|GetMiniGameWidget)) CompleteCurrent CompleteMax Timer))

(event Custom|SetVROffset
  (params (WidgetVROffset :type Float%20%28single-precision%29) (GameVROffset :type Float%20%28single-precision%29))
  ;[1 1 1] Set offset for Game Root and UI widget (used for VR)
  (Transformation|SetRelativeLocation (Variables|Default|GetScene) (Math|Vector|MakeVector WidgetVROffset 0.0 0.0) false false)
  (Transformation|SetRelativeLocation (Variables|Default|GetGameRoot) (Math|Vector|MakeVector GameVROffset 0.0 0.0) false false))

(event Custom|SetOcclusionColor
  (params (Color :type Linear%20Color%20Structure))
  (bind _occlusionspherematerialinst (Variables|Default|GetOcclusionSphereMaterialInst))
  ;[1 1 1] Set Occlusion sphere color (RGB). Pass parameter to material
  (Utilities|IsValid _occlusionspherematerialinst
    (:Is%20Valid
      (Rendering|Material|SetVectorParameterValue _occlusionspherematerialinst "Color" Color :!class /Script/Engine.MaterialInstanceDynamic))))

(event Custom|SetInfoVisibility
  (params (CompleteCount :type Integer) (TimerHide :type Boolean))
  ;[1 1 1] Set Complete and Timer visibility. Use Interface
  (Class|IMiniGameWidgetInteface|SetWidgetVisibility(Message) (UserInterface|GetUserWidgetObject (Variables|Default|GetMiniGameWidget)) CompleteCount TimerHide))

(event Custom|SetHelpText
  (params (HelpText :type Text))
  ;[1 1 1] Set Help Text. Use Interface
  (Class|IMiniGameWidgetInteface|SetWidgetHelpText(Message) (UserInterface|GetUserWidgetObject (Variables|Default|GetMiniGameWidget)) HelpText))

(event Custom|SetFadeOpacity
  (params (Opacity :type Float%20%28single-precision%29))
  (bind _fadespherematerialinst (Variables|Default|GetFadeSphereMaterialInst))
  ;[1 1 1] Set fade color opacity. Used for fadeon effect. Pass parameter to material
  (Utilities|IsValid _fadespherematerialinst
    (:Is%20Valid
      (Rendering|Material|SetScalarParameterValue _fadespherematerialinst "Opacity" Opacity :!class /Script/Engine.MaterialInstanceDynamic))))

(event Custom|HideImage
  (params (IsHide :type Boolean))
  ;[1 1 1] Show / Hide background image
  (Development|SetHiddeninGame (Variables|Default|GetBackgroundImage) IsHide false))

(event EventBeginPlay)

(event Collision|EventActorBeginOverlap
  (params (OtherActor :type Actor%20Object%20Reference)))

(event EventTick
  (params (DeltaSeconds :type Float%20%28single-precision%29)))

(fn ConstructionScript)