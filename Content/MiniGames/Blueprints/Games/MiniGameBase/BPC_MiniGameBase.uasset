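; Base component for minigames that handles activation, play, win/fail and exit, leaving spawning and input responses to child games.
; BeginPlay spawns an interact actor with a widget; activating while overlapped switches the view to the child-spawned render actor, with VR offsets.
; A Tick state machine drives fade-in, key polling, timer and completion checks, and final sounds.
; Exit waits for the child's ProcessToExit before restoring camera and pawn input, which UsePawnLogic can leave to the pawn.
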(event Custom|MiniGame_Activate
  (bind _returnvalue (Game|GetPlayerController 0))
  (bind _bp_renderptr (Variables|Default|GetBP_RenderPtr))
  ;[1 1 1] Activate MiniGame. Spawn requried BP_Render, set UI widget text and visibility, reset all variables to default. Set VR offset if run in the HMD. Switch from Pawn camera to MiniGame camera. If render not spawned then show error
  (if (Variables|GameGeneral|GetAlwaysRestartGame)
    (if (not (Variables|Default|GetGameSpawned)) :!label _label
      (CallFunction|DisablePawnInput)
      (Variables|Default|SetGameSpawned false)
      (CallFunction|SpawnMiniGame)
      (if (Variables|Default|GetGameSpawned)
        (Default|HideImage _bp_renderptr (Variables|GameGeneral|GetHideImage))
        (Variables|Default|SetGameStatus "NewEnumerator2")
        (if (Class|HeadMountedDisplayFunctionLibrary|IsHeadMountedDisplayEnabled)
          (Default|SetVROffset _bp_renderptr (Variables|GameGeneral|GetWidgetVROffset) (Variables|GameGeneral|GetGameVROffset))
          (Class|HeadMountedDisplayFunctionLibrary|ResetOrientationandPosition 0.0 "OrientationAndPosition")
          (Default|HideImage _bp_renderptr true))
        (Variables|Default|SetCurrentCompleted 0)
        (Variables|Default|SetCurrentTime (Variables|GameGeneral|GetTimer))
        (Default|CreateDynamicMaterial _bp_renderptr)
        (Default|SetOcclusionColor _bp_renderptr (Variables|GameGeneral|GetBackgroundColor))
        (Default|SetFadeOpacity _bp_renderptr 1.0)
        (Default|SetInfoValues _bp_renderptr (Variables|Default|GetCurrentCompleted) (Variables|Default|GetNeedToComplete) 1e+02)
        (Default|SetInfoVisibility _bp_renderptr (Variables|Default|GetNeedToComplete) (Variables|GameGeneral|GetUseTimer))
        (Default|SetHelpText _bp_renderptr (Variables|GameGeneral|GetHelpText))
        (Variables|Default|SetPlayerViewTarget (Pawn|GetViewTarget _returnvalue))
        (Game|Player|SetViewTargetwithBlend _returnvalue _bp_renderptr 0.0 "VTBlend_Linear" 0.0 false)
        (Variables|Default|SetIsFirstTick true)
        (Variables|Default|SetFadeCounter 0.0)
        (Variables|Default|SetWantExit false)
        (Variables|Default|SetProcessToExit false)
        (Variables|Default|SetIsGameComplete false)
        (Variables|Default|SetMiniGameState "NewEnumerator6")))
    (elif (not (Utilities|Enum|Equal(Enum) (Variables|Default|GetGameStatus) "NewEnumerator0"))
      (goto _label))))

(event Custom|MiniGame_Exit
  ;[1 1 1] Exit from the Mini Game
  (if (and (Utilities|Enum|Equal(Enum) (Variables|Default|GetMiniGameState) "NewEnumerator1") (not (Variables|Default|GetWantExit)))
    (if (Variables|GameGeneral|GetCanExit)
      (Variables|Default|SetWantExit true)
      (Variables|Default|SetMiniGameState "NewEnumerator7"))))

(event Custom|MiniGame_Toggle
  ;[1 1 1] Control Keys
  (CallFunction|TogglePressed))

(event Custom|MiniGame_Left
  ;[1 1 1] Control Keys
  (CallFunction|LeftPressed))

(event Custom|MiniGame_Right
  ;[1 1 1] Control Keys
  (CallFunction|RightPressed))

(event Custom|MiniGame_Up
  ;[1 1 1] Control Keys
  (CallFunction|UpPressed))

(event Custom|MiniGame_Down
  ;[1 1 1] Control Keys
  (CallFunction|DownPressed))

(event Custom|MiniGame_SetComplete
  ;[0.03119 1 0.1322] FOR EXTERNAL USE!
  ;;[1 1 1] Use this event if you need set complete game status. Helpful for Load / Save system
  (Variables|Default|SetGameStatus "NewEnumerator0"))

(event Custom|MiniGame_Reset
  ;[0.03119 1 0.1322] FOR EXTERNAL USE!
  ;;[1 1 1] Restart game. Call this event if you need restart game
  (Variables|Default|SetGameStatus "NewEnumerator3")
  (Default|MiniGameHideWidget (Variables|Default|GetInteractActor) false))

(event EventBeginPlay
  ;[1 1 1] Spawn once on start Interact Actor and add specified UI widget with requred parameters - sphere radius, use hemisphere, widget scale
  (Variables|Default|SetActivatePressed false)
  (Variables|Default|SetGameStatus "NewEnumerator3")
  (Variables|Default|SetGameSpawned false)
  (bind _returnvalue (Game|SpawnActorfromClass "/Game/MiniGames/Blueprints/Games/MiniGameBase/BP_MiniGameInteractActor.BP_MiniGameInteractActor_C" (Transformation|GetWorldTransform) "Undefined" (Components|GetOwner) 0))
  (bind _output_get (Variables|Default|SetInteractActor _returnvalue))
  (Default|MiniGameCreateWidget _output_get (Variables|InteractionWidget|GetInteractWidget) (.Key (Utilities|Struct|BreakInputActionKeyMapping (Utilities|Array|Get(acopy) (Variables|InteractionKeys|GetActivateGame)))) (Variables|InteractionWidget|GetScale) (Variables|InteractionWidget|GetUseHemisphere) (Variables|InteractionWidget|GetInteractRadius)))

(event EventTick
  (params (DeltaSeconds :type Float%20%28single-precision%29))
  (bind _activategame (Variables|InteractionKeys|GetActivateGame))
  ;[1 1 1] Main state machine
  (switch Utilities|FlowControl|Switch|SwitchonE_MiniGameState (Variables|Default|GetMiniGameState)
    (:NewEnumerator0
      (if (not (Variables|InteractionKeys|GetUsePawnLogic))
        ;;[0 0.8909 1] Check if Activate game pressed
        (Variables|Default|SetActivatePressed false)
        (for (_ _array_index) _activategame
          (if (Game|Player|IsInputKeyDown (Game|GetPlayerController 0) (.Key (Utilities|Struct|BreakInputActionKeyMapping (Utilities|Array|Get(acopy) _activategame _array_index))))
            (Variables|Default|SetActivatePressed true)))
        (bind _pawninside (CallFunction|GetPawnOverlapped))
        (if (and _pawninside (Variables|Default|GetActivatePressed))
          (CallFunction|MiniGameActivate))))
    (:NewEnumerator1
      (CallFunction|CheckKeys)
      (if (Variables|Default|GetGameSpawned)
        ;;[0 0.8909 1] Check keys,, calculate time and pass values to UI widget
        (CallFunction|CheckAttepmtCompleteTime)
        (CallFunction|CalculateTimer)
        (Default|SetInfoValues (Variables|Default|GetBP_RenderPtr) (Variables|Default|GetCurrentCompleted) (Variables|Default|GetNeedToComplete) (/ (* (Variables|Default|GetCurrentTime) 1e+02) (Variables|GameGeneral|GetTimer)))))
    (:NewEnumerator3
      (CallFunction|PlayFinalSound (Variables|GameGeneral|GetFailedSound))
      (Variables|Default|SetMiniGameState "NewEnumerator8"))
    (:NewEnumerator4
      (CallFunction|PlayFinalSound (Variables|GameGeneral|GetSuccessSound))
      (Variables|Default|SetMiniGameState "NewEnumerator8"))
    (:NewEnumerator2
      ;;[0 0.8909 1] Exit from MiniGame. Destroy render actor and switch camera to Pawn camera
      (CallFunction|StopSounds)
      (Game|Player|SetViewTargetwithBlend (Game|GetPlayerController 0) (Variables|Default|GetPlayerViewTarget) 0.0 "VTBlend_Linear" 0.0 false)
      (Actor|DestroyActor (Variables|Default|GetBP_RenderPtr))
      (CallFunction|EnablePawnInput)
      (Variables|Default|SetGameSpawned false)
      (Variables|Default|SetMiniGameState "NewEnumerator0"))
    (:NewEnumerator6
      ;;[0 0.8909 1] FadeIn effect
      (Default|SetFadeOpacity (Variables|Default|GetBP_RenderPtr) (- 1.0 (Math|Float|Clamp(Float) (+ (* DeltaSeconds (Variables|GameGeneral|GetFadeSpeed)) (Variables|Default|GetFadeCounter)))))
      (Variables|Default|SetFadeCounter (Math|Float|Clamp(Float) (+ (* DeltaSeconds (Variables|GameGeneral|GetFadeSpeed)) (Variables|Default|GetFadeCounter))))
      (if (>= (Math|Float|Clamp(Float) (+ (* DeltaSeconds (Variables|GameGeneral|GetFadeSpeed)) (Variables|Default|GetFadeCounter))) 1.0)
        (Variables|Default|SetMiniGameState "NewEnumerator1")))
    (:NewEnumerator7
      ;;[0 0.8909 1] If parent MiniGame ready to exit (ProcessToExit = true) then switch to Exit state
      (if (Variables|Default|GetProcessToExit)
        (Variables|Default|SetMiniGameState "NewEnumerator2")))
    (:NewEnumerator8
      ;;[0 0.8909 1] Wait while final sound is playing
      (if (>= (- (Utilities|Time|GetGameTimeinSeconds) (Variables|Default|GetFinalSoundStartTime)) (Variables|Default|GetFinalSoundDuration))
        (Variables|Default|SetWantExit true)
        (Variables|Default|SetMiniGameState "NewEnumerator7")))))

(fn CheckKeys
  ;[1 1 1] Check dafined keys on pressed state. All keys stored in the Ineraction keys variables. If key pressed then call relevant event
  (if (not (Variables|InteractionKeys|GetUsePawnLogic))
    (Utilities|FlowControl|Sequence
      (:then_0
        (LocalVariables|SetbActivateKeyDetected false)
        (LocalVariables|SetbExitKeyDetected false)
        (LocalVariables|SetbToggleKeyDetected false)
        (LocalVariables|SetbLeftKeyDetected false)
        (LocalVariables|SetbRightKeyDetected false)
        (LocalVariables|SetbUpKeyDetected false)
        (LocalVariables|SetbDownKeyDetected false)
        (CallFunction|TestKey (Variables|InteractionKeys|GetActivateGame) (LocalVariables|GetbActivateKeyDetected) 1.0)
        (CallFunction|TestKey (Variables|InteractionKeys|GetExitFromGame) (LocalVariables|GetbExitKeyDetected) 1.0)
        (CallFunction|TestKey (Variables|InteractionKeys|GetSelect) (LocalVariables|GetbToggleKeyDetected) 1.0)
        (CallFunction|TestKey (Variables|InteractionKeys|GetLeft) (LocalVariables|GetbLeftKeyDetected) -1.0)
        (CallFunction|TestKey (Variables|InteractionKeys|GetRight) (LocalVariables|GetbRightKeyDetected) 1.0)
        (CallFunction|TestKey (Variables|InteractionKeys|GetUp) (LocalVariables|GetbUpKeyDetected) 1.0)
        (CallFunction|TestKey (Variables|InteractionKeys|GetDown) (LocalVariables|GetbDownKeyDetected) -1.0))
      (:then_1
        (if (LocalVariables|GetbActivateKeyDetected)
          (CallFunction|MiniGameActivate)))
      (:then_2
        (if (LocalVariables|GetbExitKeyDetected)
          (CallFunction|MiniGameExit)))
      (:then_3
        (if (LocalVariables|GetbToggleKeyDetected)
          (CallFunction|MiniGameToggle)))
      (:then_4
        (if (LocalVariables|GetbLeftKeyDetected)
          (CallFunction|MiniGameLeft)))
      (:then_5
        (if (LocalVariables|GetbRightKeyDetected)
          (CallFunction|MiniGameRight)))
      (:then_6
        (if (LocalVariables|GetbUpKeyDetected)
          (CallFunction|MiniGameUp)))
      (:then_7
        (if (LocalVariables|GetbDownKeyDetected)
          (CallFunction|MiniGameDown))))))

(fn TestKey
  (params (KeyMapping :type Array%20of%20Input%20Action%20Key%20Mapping%20Structures) (KeyResult :type Boolean%20%28by%20ref%29) (Mask :type Float%20%28single-precision%29))
  (bind _returnvalue (Game|GetPlayerController 0))
  ;[1 1 1] Test key if pressed. All keys get from key mapping array stored in the Interaction Keys
  (for _array_element KeyMapping
    (if (Game|Player|WasInputKeyJustPressed _returnvalue (.Key (Utilities|Struct|BreakInputActionKeyMapping _array_element)))
      ;;[0 0.9409 1] If gamepad used then test with requred mask
      (if (Class|KismetInputLibrary|KeyIsGamepadKey (.Key (Utilities|Struct|BreakInputActionKeyMapping _array_element)))
        (if (== (Math|Float|Sign(Float) Mask) (Math|Float|Sign(Float) (Class|PlayerController|GetInputAnalogKeyState _returnvalue (.Key (Utilities|Struct|BreakInputActionKeyMapping _array_element)))))
          (|SetBy-RefVar KeyResult true :!label _label))
        (else
          (goto _label))))))

(fn SpawnMiniGame
  ;[1 1 1] Spawn MiniGame. Called inside of parent game
)

(fn ExitPressed
  ;[1 1 1] Exit pressed
)

(fn TogglePressed
  ;[1 1 1] Select pressed. Called inside of parent game
)

(fn LeftPressed
  ;[1 1 1] Left pressed. Called inside of parent game
)

(fn RightPressed
  ;[1 1 1] Right pressed. Called inside of parent game
)

(fn UpPressed
  ;[1 1 1] Up pressed. Called inside of parent game
)

(fn DownPressed
  ;[1 1 1] Down pressed. Called inside of parent game
)

(fn PlaySoundFX
  (params (SoundFx :type Sound%20Wave%20Object%20Reference) (StartTime :type Float%20%28single-precision%29) (Active :type Boolean))
  ;[1 1 1] Play wav sound with specified start time and activate flag via Sound 2D. Return spawned audio component ref
  (bind _returnvalue (Audio|SpawnSound2D SoundFx 1.0 1.0 StartTime 0))
  (Components|Activation|SetActive _returnvalue Active true)
  (return _returnvalue))

(fn CalculateTimer
  ;[1 1 1] Calculate MiniGame timer. How much time left from start
  (if (Variables|Default|GetIsFirstTick)
    (Variables|Default|SetStartTickTime (Utilities|Time|GetGameTimeinSeconds))
    (Variables|Default|SetIsFirstTick false))
  (Variables|Default|SetCurrentTime (Math|Float|Clamp(Float) (- (Variables|GameGeneral|GetTimer) (- (Utilities|Time|GetGameTimeinSeconds) (Variables|Default|GetStartTickTime))) 0.0 1e+03)))

(fn IncreaseComplete
  ;[1 1 1] Increase Complete value
  (Variables|Default|SetCurrentCompleted (+ (Variables|Default|GetCurrentCompleted) 1)))

(fn CheckAttepmtCompleteTime
  (bind _needtocomplete (Variables|Default|GetNeedToComplete))
  ;[1 1 1] Check conditions for timer, completed value and game complete
  (switch Utilities|FlowControl|Switch|SwitchonE_MiniGameState (Variables|Default|GetMiniGameState)
    (:NewEnumerator1
      (Utilities|FlowControl|Sequence
        (:then_0
          (if (and (<= (Variables|Default|GetCurrentTime) 0.1) (Variables|GameGeneral|GetUseTimer))
            (Variables|Default|SetMiniGameState "NewEnumerator3")
            (Variables|Default|SetGameStatus "NewEnumerator1")))
        (:then_1
          (if (> _needtocomplete 0)
            (if (>= (Variables|Default|GetCurrentCompleted) _needtocomplete)
              (Variables|Default|SetMiniGameState "NewEnumerator4" :!label _label)
              (Variables|Default|SetGameStatus "NewEnumerator0")
              (if (not (Variables|GameGeneral|GetAlwaysRestartGame))
                (Default|MiniGameHideWidget (Variables|Default|GetInteractActor) true)))))
        (:then_2
          (if (Variables|Default|GetIsGameComplete)
            (goto _label)))))))

(fn PlayFinalSound
  (params (Sound :type Sound%20Cue%20Object%20Reference))
  ;[1 1 1] Play final Good or Bad sound
  (Utilities|IsValid Sound
    (:Is%20Valid
      (CallFunction|PlaySoundCue Sound 0.0)
      (Variables|Default|SetFinalSoundDuration (Variables|/Script/Engine.SoundBase|GetDuration Sound)))
    (:Is%20Not%20Valid
      (Variables|Default|SetFinalSoundDuration 0.0)))
  (Variables|Default|SetFinalSoundStartTime (Utilities|Time|GetGameTimeinSeconds)))

(fn DisablePawnInput
  ;[1 1 1] Disable input for Pawn. When game is started we need block any player inputs if not used Pawn logic
  (if (not (Variables|InteractionKeys|GetUsePawnLogic))
    (Input|DisableInput (Game|Player|GetPlayerPawn 0) (Game|GetPlayerController 0))))

(fn EnablePawnInput
  ;[1 1 1] Enable Pawn input
  (if (not (Variables|InteractionKeys|GetUsePawnLogic))
    (Input|EnableInput (Game|Player|GetPlayerPawn 0) (Game|GetPlayerController 0))))

(fn GetGameStatus
  ;[1 1 1] Return game status: Success - game is succesfuly completed. Failed - not complete (rejected by timer). Play / Idle - working state
  (return (Variables|Default|GetGameStatus)))

(fn SetRenderPtr
  (params (RenderPtr :type BP%20Render%20Base%20Object%20Reference))
  ;[1 1 1] Store MiniGame render ref pointer
  (Variables|Default|SetBP_RenderPtr RenderPtr))

(fn SetGameSpawned
  (params (Spawned :type Boolean))
  ;[1 1 1] Set game spawned value
  (Variables|Default|SetGameSpawned Spawned))

(fn GetGameSpawned
  ;[1 1 1] Get game spawned value
  (return (Variables|Default|GetGameSpawned)))

(fn GetPawnOverlapped
  ;[1 1 1] Check if any Pawn currently overlapped with MiniGame
  (bind _ispawnoverlapped (Default|GetIsPawnOverlapped (Variables|Default|GetInteractActor)))
  (return _ispawnoverlapped))

(fn GetAnchorTransform
  ;[1 1 1] Get MiniGame Anchor object on the map. If Anchor not found then show error otherwise return Anchor transform
  (bind _outactors (Actor|GetAllActorsOfClass "/Game/MiniGames/Blueprints/Games/BP_MiniGameAnchor.BP_MiniGameAnchor_C"))
  (Utilities|IsValid (Utilities|Array|Get(acopy) _outactors)
    (:Is%20Valid
      (LocalVariables|SetTransform (Math|Transform|MakeTransform (Transformation|GetActorLocation (Utilities|Array|Get(acopy) _outactors))))
      (LocalVariables|SetResult true))
    (:Is%20Not%20Valid
      (Development|PrintString "Error: No BP_MiniGameAnchor found on the level!" true true "(R=1.000000,G=0.000000,B=0.000000,A=1.000000)" 5.0)
      (LocalVariables|SetResult false)))
  (return (LocalVariables|GetTransform) (LocalVariables|GetResult)))

(fn PlaySoundCue
  (params (SoudCue :type Sound%20Cue%20Object%20Reference) (StartTime :type Float%20%28single-precision%29))
  ;[1 1 1] Play sound Cue and store spawned Sound 2D ref in the array
  (bind _returnvalue (Audio|SpawnSound2D SoudCue 1.0 1.0 StartTime 0))
  (Utilities|Array|Add (Variables|Default|GetAudioCompArray) _returnvalue)
  (return _returnvalue))

(fn SetNeedtoComplete
  (params (Value :type Integer))
  ;[1 1 1] Store need to Complete value. E.g. need found 2 quality in the Fast Lock game
  (Variables|Default|SetNeedToComplete Value))

(fn DecreaseComplete
  ;[1 1 1] Decrease Complete value. Max value is 5
  (Variables|Default|SetCurrentCompleted (Math|Integer|Clamp(Integer) (- (Variables|Default|GetCurrentCompleted) 1) 0 5)))

(fn StopSounds
  ;[1 1 1] Stop spawned Sound 2d stored in the PlaySoundCue method
  (for _array_element (Variables|Default|GetAudioCompArray)
    (Utilities|IsValid _array_element
      (:Is%20Valid
        (Audio|Components|Audio|Stop _array_element)))))

(fn GetMiniGameState
  ;[1 1 1] Get MiniGames state. Helper function
  (return (Variables|Default|GetMiniGameState)))

(fn GetWantExit
  ;[1 1 1] Get WantExit value. If true - player press exit button
  (return (Variables|Default|GetWantExit)))

(fn SetProcesstoExit
  (params (ToExit :type Boolean))
  ;[1 1 1] Set ProceesToExit value
  (Variables|Default|SetProcessToExit ToExit))

(fn SetGameComplete
  ;[1 1 1] Set CompleteGame value. This value set only parent game
  (Variables|Default|SetIsGameComplete true))