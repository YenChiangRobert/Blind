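; BP_FinderRender is the visual actor for the Finder minigame, drawing its cells, symbol caps and selector.
; SpawnCell adds cell and cap meshes at runtime, picking each cap's symbol through UV offsets on a dynamic material instance, and records the cap by ID.
; Helper functions then rotate, scale or hide caps by ID, move, scale or hide the selector, toggle the central cell, and report cell size.
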(event EventBeginPlay
  (|CallParentFunction)
  ;[1 1 1] Store Cell mesh size
  (Variables|Default|SetCellSize (* (.Z (Math|Vector|BreakVector (.BoxExtent (Math|BoxSphereBounds|BreakBoxSphereBounds (StaticMesh|GetBounds (Variables|Default|GetMeshCell)))))) 2.0)))

(event Collision|EventActorBeginOverlap
  (params (OtherActor :type Actor%20Object%20Reference)))

(event EventTick
  (params (DeltaSeconds :type Float%20%28single-precision%29)))

(fn ConstructionScript
  (|CallParentFunction))

(fn GetCellSize
  ;[1 1 1] Return Cell size
  (return (Variables|Default|GetCellSize)))

(fn SpawnCell
  (params (CellData :type S%20Finder%20Data%20Structure))
  (bind (_id _capmeshcomponent _location _cellnumber _isactive) (Utilities|Struct|BreakS_FinderData CellData))
  (bind _uvcaps (Variables|Default|GetUVCaps))
  (bind _item (Utilities|Array|Get(acopy) _uvcaps _cellnumber))
  (bind _returnvalue (Math|Transform|MakeTransform _location "0,0.000000,0.000000" "1,1,1.000000"))
  (bind (_x _y) (Math|Vector2D|BreakVector2D _item))
  ;[1 1 1] Add static mesh component. Set Cap mesh. Create dynamic material and pass UV offset params into material. UV offset specified for each symbol on the texture
  (bind _returnvalue_2 (AddComponent|AddStaticMeshComponent false _returnvalue))
  (Components|StaticMesh|SetStaticMesh _returnvalue_2 (Variables|Default|GetMeshCell))
  (Transformation|AttachComponentToComponent _returnvalue_2 (Variables|Default|GetFinderRoot) "None" "KeepRelative" "KeepRelative" "KeepRelative" true)
  (bind _returnvalue_3 (AddComponent|AddStaticMeshComponent false _returnvalue))
  (bind _returnvalue_4 (Rendering|Material|CreateDynamicMaterialInstance "/Game/MiniGames/Materials/Finder/M_FinderCap.M_FinderCap" :!class /Script/Engine.KismetMaterialLibrary))
  (Rendering|Material|SetMaterial _returnvalue_3 0 _returnvalue_4)
  (Rendering|Material|SetScalarParameterValue _returnvalue_4 "UOffset" _x :!class /Script/Engine.MaterialInstanceDynamic)
  (Rendering|Material|SetScalarParameterValue _returnvalue_4 "VOffset" _y :!class /Script/Engine.MaterialInstanceDynamic)
  (Components|StaticMesh|SetStaticMesh _returnvalue_3 (Variables|Default|GetMeshCap))
  (Transformation|AttachComponentToComponent _returnvalue_3 (Variables|Default|GetFinderRoot) "None" "KeepRelative" "KeepRelative" "KeepRelative" true)
  (Utilities|Array|Add (Variables|Default|GetCellsArray) (Utilities|Struct|MakeS_FinderData _id _returnvalue_3 _location _cellnumber _isactive)))

(fn HideCentralCell
  (params (Show :type Boolean))
  ;[1 1 1] Helper function. Hide central cell mesh
  (Development|SetHiddeninGame (Variables|Default|GetSM_FinderCell) Show false))

(fn SetSelectorLocation
  (params (Location :type Vector))
  ;[1 1 1] Set relative location for selector mesh
  (Transformation|SetRelativeLocation (Variables|Default|GetSM_FinderSelector) Location false false))

(fn HideSelector
  (params (Hide :type Boolean))
  ;[1 1 1] Helper function. Hide selector mesh
  (Development|SetHiddeninGame (Variables|Default|GetSM_FinderSelector) Hide false))

(fn SetCellParameters
  (params (CellId :type Integer) (RotZ :type Float%20%28single-precision%29) (Scale :type Float%20%28single-precision%29) (Hide :type Boolean))
  ;[1 1 1] Set dynamic parameters for Cell specified by Cell_ID
  (bind _array_element (Utilities|Array|ForEachLoopwithBreak (Variables|Default|GetCellsArray) :!label _label)
    (:LoopBody
      (if (== CellId (.Id (Utilities|Struct|BreakS_FinderData _array_element)))
        (goto _label Break)))
    (:Completed
      (Transformation|SetRelativeRotation (.CapMeshComponent (Utilities|Struct|BreakS_FinderData _array_element)) (Math|Rotator|MakeRotator 0.0 0.0 RotZ) false false)
      (Transformation|SetRelativeScale3D (.CapMeshComponent (Utilities|Struct|BreakS_FinderData _array_element)) (Math|Vector|MakeVector Scale Scale Scale))
      (Development|SetHiddeninGame (.CapMeshComponent (Utilities|Struct|BreakS_FinderData _array_element)) Hide false))))

(fn SetSelectorScale
  (params (Scake :type Float%20%28single-precision%29))
  ;[1 1 1] Helper function. Set selector mesh relative scale
  (Transformation|SetRelativeScale3D (Variables|Default|GetSM_FinderSelector) (Math|Vector|MakeVector Scake 1.0 Scake)))