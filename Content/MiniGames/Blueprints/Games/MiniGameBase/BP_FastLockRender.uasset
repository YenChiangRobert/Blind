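; Render actor for the FastLock minigame, displaying a lock built from sixteen segment meshes plus a finish segment under a rotating root.
; BeginPlay caches initial segment and root transforms as the base for later movement.
; Setters swap meshes, rotate the root, and slide the start segment, segments 1 and 15, and the finish segment along their own directions.
; Getters expose the start segment's length and location and the finish segment's location.
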(event EventBeginPlay
  ;[1 1 1] Store initial rotation for segmantes and root rotation
  (Variables|Default|SetSeg1_InitPitchRotation (.Pitch (Math|Rotator|BreakRotator (Variables|/Script/Engine.SceneComponent|GetRelativeRotation (Variables|Default|GetSeg1)))))
  (Variables|Default|SetSeg15_InitPitchRotation (.Pitch (Math|Rotator|BreakRotator (Variables|/Script/Engine.SceneComponent|GetRelativeRotation (Variables|Default|GetSeg15)))))
  (Variables|Default|SetSegFinish_InitLocation (Variables|/Script/Engine.SceneComponent|GetRelativeLocation (Variables|Default|GetSegFinish)))
  (Variables|Default|SetRootInitRotation (Variables|/Script/Engine.SceneComponent|GetRelativeRotation (Variables|Default|GetLockRoot)))
  (Variables|Default|SetRoot_InitLocation (Variables|/Script/Engine.SceneComponent|GetRelativeLocation (Variables|Default|GetLockRoot))))

(fn ConstructionScript)

(fn SetSegmentMesh
  (params (Index :type Integer) (Mesh :type Static%20Mesh%20Object%20Reference))
  ;[1 1 1] Set specified mesh by index for Lock segment. Total is 16 meshes
  (LocalVariables|SetSegmentMesh Mesh)
  (switch int Index
    (:0
      (LocalVariables|SetMeshComponent (Variables|Default|GetSeg0)))
    (:1
      (LocalVariables|SetMeshComponent (Variables|Default|GetSeg1)))
    (:2
      (LocalVariables|SetMeshComponent (Variables|Default|GetSeg2)))
    (:3
      (LocalVariables|SetMeshComponent (Variables|Default|GetSeg3)))
    (:4
      (LocalVariables|SetMeshComponent (Variables|Default|GetSeg4)))
    (:5
      (LocalVariables|SetMeshComponent (Variables|Default|GetSeg5)))
    (:6
      (LocalVariables|SetMeshComponent (Variables|Default|GetSeg6)))
    (:7
      (LocalVariables|SetMeshComponent (Variables|Default|GetSeg7)))
    (:8
      (LocalVariables|SetMeshComponent (Variables|Default|GetSeg8)))
    (:9
      (LocalVariables|SetMeshComponent (Variables|Default|GetSeg9)))
    (:10
      (LocalVariables|SetMeshComponent (Variables|Default|GetSeg10)))
    (:11
      (LocalVariables|SetMeshComponent (Variables|Default|GetSeg11)))
    (:12
      (LocalVariables|SetMeshComponent (Variables|Default|GetSeg12)))
    (:13
      (LocalVariables|SetMeshComponent (Variables|Default|GetSeg13)))
    (:14
      (LocalVariables|SetMeshComponent (Variables|Default|GetSeg14)))
    (:15
      (LocalVariables|SetMeshComponent (Variables|Default|GetSeg15))))
  (Components|StaticMesh|SetStaticMesh (LocalVariables|GetMeshComponent) (LocalVariables|GetSegmentMesh)))

(fn SetMeshOffset
  (params (SegIndex :type Integer) (Offset :type Float%20%28single-precision%29))
  ;[1 1 1] Set relative offsets for Start, Final and next segments
  (LocalVariables|SetRelativeOffset (Math|Vector|MakeVector Offset 0.0 0.0))
  (switch int SegIndex
    (:0
      (Transformation|SetRelativeLocation (Variables|Default|GetSeg0) (LocalVariables|GetRelativeOffset) false false))
    (:1
      (Transformation|SetRelativeLocation (Variables|Default|GetSeg1) (Math|Vector|RotateVector (LocalVariables|GetRelativeOffset) (Math|Rotator|MakeRotator 0.0 (Variables|Default|GetSeg1_InitPitchRotation) 0.0)) false false))
    (:2
      (Transformation|SetRelativeLocation (Variables|Default|GetSeg15) (Math|Vector|RotateVector (LocalVariables|GetRelativeOffset) (Math|Rotator|MakeRotator 0.0 (Variables|Default|GetSeg15_InitPitchRotation) 0.0)) false false))
    (:3
      (Transformation|SetRelativeLocation (Variables|Default|GetSegFinish) (+ (Variables|Default|GetSegFinish_InitLocation) (* (Math|Vector|Normalize (- (Variables|Default|GetSegFinish_InitLocation) (Variables|Default|GetRoot_InitLocation))) (.X (Math|Vector|BreakVector (LocalVariables|GetRelativeOffset))))) false false))))

(fn RotateRoot
  (params (Angle :type Float%20%28single-precision%29))
  (bind _rootinitrotation (Variables|Default|GetRootInitRotation))
  ;[1 1 1] Rotate Lock root around pitch axis
  (Transformation|SetRelativeRotation (Variables|Default|GetLockRoot) (Math|Rotator|CombineRotators _rootinitrotation (Math|Vector|RotatorfromAxisandAngle (.Y (Math|Rotator|BreakRotIntoAxes _rootinitrotation)) (* Angle -1.0))) false false))

(fn SetFinishSegmentMesh
  (params (Mesh :type Static%20Mesh%20Object%20Reference))
  ;[1 1 1] Set mesh for Finish segment
  (Components|StaticMesh|SetStaticMesh (Variables|Default|GetSegFinish) Mesh))

(fn GetStartSegLengthLocation
  (bind _seg0 (Variables|Default|GetSeg0))
  ;[1 1 1] Get size and init location of Start segment
  (return (.X (Math|Vector|BreakVector (.Max (Components|StaticMesh|GetLocalBounds _seg0)))) (Transformation|GetWorldLocation _seg0)))

(fn GetFinishSegLocation
  ;[1 1 1] Get Finish segment location
  (return (Transformation|GetWorldLocation (Variables|Default|GetSegFinish))))