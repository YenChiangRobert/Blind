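; Interaction point actor for minigames that shows a prompt widget and reports whether a pawn is in range.
; Setup creates the given widget on its widget component, scales it and sets the trigger sphere radius; another event toggles widget visibility.
; Overlap events cache the first overlapping pawn and clear it once none remain in the sphere.
; GetIsPawnOverlapped returns that state, or in hemisphere mode uses a dot-product angle test to accept only pawns in front.
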(event Custom|MiniGame_CreateWidget
  (params (InteractWidget :type User%20Widget%20Class%20Reference) (Key :type Key%20Structure :default "None") (Scale :type Vector%202D%20Structure) (UseHemisphere :type Boolean) (SphereRadius :type Float%20%28single-precision%29))
  (bind _returnvalue (UserInterface|CreateWidget InteractWidget))
  (UserInterface|SetWidget (Variables|Default|GetWidget) _returnvalue)
  (Widget|Transform|SetRenderScale _returnvalue Scale)
  (Variables|Default|SetUseHemisphere UseHemisphere)
  (Components|Sphere|SetSphereRadius (Variables|Default|GetSphere) SphereRadius true)
  (Variables|Default|SetMaxAngle 9e+01))

(event Custom|MiniGame_HideWidget
  (params (Hide :type Boolean))
  (Development|SetHiddeninGame (Variables|Default|GetWidget) Hide false))

(event Collision|EventActorBeginOverlap
  (params (OtherActor :type Actor%20Object%20Reference))
  (bind _overlappingactors (Collision|GetOverlappingActors "/Script/Engine.Pawn" :!class /Script/Engine.Actor))
  (if (> (Utilities|Array|Length _overlappingactors) 0)
    (Variables|Default|SetPawnActor (Utilities|Array|Get(acopy) _overlappingactors))
    (Variables|Default|SetIsPawnOverlapped true)))

(event Collision|EventActorEndOverlap
  (params (OtherActor :type Actor%20Object%20Reference))
  (if (and (Variables|Default|GetIsPawnOverlapped) (== (Utilities|Array|Length (Collision|GetOverlappingActors (Variables|Default|GetSphere) "/Script/Engine.Pawn" :!class /Script/Engine.PrimitiveComponent)) 0))
    (Variables|Default|SetIsPawnOverlapped false)
    (Variables|Default|SetPawnActor 0)))

(fn ConstructionScript)

(fn GetIsPawnOverlapped
  (bind _defaultsceneroot (Variables|Default|GetDefaultSceneRoot))
  (bind _returnvalue (Transformation|GetWorldTransform _defaultsceneroot))
  (bind (_location _rotation) (Math|Transform|BreakTransform _returnvalue))
  (LocalVariables|SetIsPawnInside false)
  (if (Variables|Default|GetUseHemisphere)
    (Utilities|IsValid (Variables|Default|GetPawnActor)
      (:Is%20Valid
        (if (<= (Class|KismetMathLibrary|DegAcos (Math|Vector|DotProduct (Math|Vector|Normalize (Math|Vector|RotateVector (- (Transformation|GetActorLocation (Variables|Default|GetPawnActor)) _location) _rotation)) (Math|Vector|Normalize (Math|Vector|RotateVector (- (+ _location (* (Math|Vector|GetForwardVector _defaultsceneroot) 5e+01)) _location) _rotation)))) (Variables|Default|GetMaxAngle))
          (LocalVariables|SetIsPawnInside true)))
      (:Is%20Not%20Valid
        _))
    (else
      (LocalVariables|SetIsPawnInside (Variables|Default|GetIsPawnOverlapped))))
  (return (LocalVariables|GetIsPawnInside)))