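; Render actor for the TriWay minigame that builds and updates its visuals: wheels, selector and beam effects.
; SpawnWheel creates a wheel mesh with three color-chosen pins 120 degrees apart, storing it in WheelsArray for later moves and rotations by index.
; SpawnPS centers a beam particle system between two points, aims its endpoints along their direction and keeps it disabled until EnablePS.
; Helpers move, scale and hide the selector.
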(event EventBeginPlay
  (|CallParentFunction)
  ;[1 1 1] Store wheel mesh size
  (Variables|Default|SetWheelSize (* (.Z (Math|Vector|BreakVector (.BoxExtent (Math|BoxSphereBounds|BreakBoxSphereBounds (StaticMesh|GetBounds (Variables|Default|GetMeshWheelBase)))))) 2.0)))

(event Collision|EventActorBeginOverlap
  (params (OtherActor :type Actor%20Object%20Reference)))

(event EventTick
  (params (DeltaSeconds :type Float%20%28single-precision%29)))

(fn ConstructionScript
  (|CallParentFunction))

(fn GetWheelSize
  ;[1 1 1] Helper function. Get Wheel mesh size
  (return (Variables|Default|GetWheelSize)))

(fn SpawnWheel
  (params (Location :type Vector) (Angle :type Float%20%28single-precision%29) (Pin0 :type E_TriWayPinColor%20Enum) (Pin1 :type E_TriWayPinColor%20Enum) (Pin2 :type E_TriWayPinColor%20Enum))
  ;[1 1 1] Spawn wheel mesh and three pins specified by pin colors and location
  (LocalVariables|SetRotAngle Angle)
  (LocalVariables|SetWheelTransform (Math|Transform|MakeTransform Location "0.000000, 0, 0" "1,1,1.000000"))
  (LocalVariables|SetPinTransform0 (Math|Transform|MakeTransform "0, 0, 0"))
  (LocalVariables|SetPinTransform1 (Math|Transform|MakeTransform "0, 0, 0" (Math|Rotator|MakeRotator 0.0 -1.2e+02 0.0)))
  (LocalVariables|SetPinTrnasfrom2 (Math|Transform|MakeTransform "0, 0, 0" (Math|Rotator|MakeRotator 0.0 -2.4e+02 0.0)))
  (LocalVariables|SetPinColor0 Pin0)
  (LocalVariables|SetPinColor1 Pin1)
  (LocalVariables|SetPinColor2 Pin2)
  (bind _returnvalue (AddComponent|AddStaticMeshComponent false (LocalVariables|GetWheelTransform)))
  (Components|StaticMesh|SetStaticMesh _returnvalue (Variables|Default|GetMeshWheelBase))
  (Transformation|AttachComponentToComponent _returnvalue (Variables|Default|GetTriWayRoot) "None" "KeepRelative" "KeepRelative" "KeepRelative" true)
  (bind _mesh (CallFunction|GetPinMesh (LocalVariables|GetPinColor0)))
  (bind _returnvalue_2 (AddComponent|AddStaticMeshComponent false (LocalVariables|GetPinTransform0)))
  (Components|StaticMesh|SetStaticMesh _returnvalue_2 _mesh)
  (Transformation|AttachComponentToComponent _returnvalue_2 _returnvalue "None" "KeepRelative" "KeepRelative" "KeepRelative" true)
  (bind _mesh_2 (CallFunction|GetPinMesh (LocalVariables|GetPinColor1)))
  (bind _returnvalue_3 (AddComponent|AddStaticMeshComponent false (LocalVariables|GetPinTransform1)))
  (Components|StaticMesh|SetStaticMesh _returnvalue_3 _mesh_2)
  (Transformation|AttachComponentToComponent _returnvalue_3 _returnvalue "None" "KeepRelative" "KeepRelative" "KeepRelative" true)
  (bind _mesh_3 (CallFunction|GetPinMesh (LocalVariables|GetPinColor2)))
  (bind _returnvalue_4 (AddComponent|AddStaticMeshComponent false (LocalVariables|GetPinTrnasfrom2)))
  (Components|StaticMesh|SetStaticMesh _returnvalue_4 _mesh_3)
  (Transformation|AttachComponentToComponent _returnvalue_4 _returnvalue "None" "KeepRelative" "KeepRelative" "KeepRelative" true)
  (Transformation|SetRelativeRotation _returnvalue (Math|Rotator|MakeRotator 0.0 (LocalVariables|GetRotAngle) 0.0) false false)
  (Utilities|Array|Add (Variables|Default|GetWheelsArray) (Utilities|Struct|MakeS_TriWayData _returnvalue "0, 0, 0")))

(fn SetSelectorLocation
  (params (Location :type Vector))
  ;[1 1 1] Set selector mesh relative location
  (Transformation|SetRelativeLocation (Variables|Default|GetSelector) Location false false))

(fn HideSelector
  (params (Hide :type Boolean))
  ;[1 1 1] Hide / Show selector mesh
  (Development|SetHiddeninGame (Variables|Default|GetSelector) Hide false))

(fn SetCellParameters
  (params (CellId :type Integer) (RotZ :type Float%20%28single-precision%29) (Scale :type Float%20%28single-precision%29) (Hide :type Boolean))
  ;[1 1 1] Set Wheel parameters specified by ID
  (bind _array_element (Utilities|Array|ForEachLoopwithBreak 0 :!label _label)
    (:LoopBody
      (if (== CellId (.Id (Utilities|Struct|BreakS_FinderData _array_element)))
        (goto _label Break)))
    (:Completed
      (Transformation|SetRelativeRotation (.CapMeshComponent (Utilities|Struct|BreakS_FinderData _array_element)) (Math|Rotator|MakeRotator 0.0 0.0 RotZ) false false)
      (Transformation|SetRelativeScale3D (.CapMeshComponent (Utilities|Struct|BreakS_FinderData _array_element)) (Math|Vector|MakeVector Scale Scale Scale))
      (Development|SetHiddeninGame (.CapMeshComponent (Utilities|Struct|BreakS_FinderData _array_element)) Hide false))))

(fn SetSelectorScale
  (params (Scake :type Float%20%28single-precision%29))
  ;[1 1 1] Helper function. Set selector mesh scale
  (Transformation|SetRelativeScale3D (Variables|Default|GetSelector) (Math|Vector|MakeVector Scake 1.0 Scake)))

(fn SpawnPS
  (params (ParticleSystem :type Particle%20System%20Object%20Reference) (SourceLocation :type Vector) (DestLocation :type Vector))
  (bind _returnvalue (- DestLocation SourceLocation))
  (bind (_x _y _z) (Math|Vector|BreakVector SourceLocation))
  (bind (_x_2 _y_2 _z_2) (Math|Vector|BreakVector DestLocation))
  (bind _beam_lenght (Variables|Default|GetBeam_Lenght))
  (bind _returnvalue_2 (Math|Vector|Normalize _returnvalue))
  (bind _returnvalue_3 (* _returnvalue_2 _beam_lenght))
  ;[1 1 1] Spawn particle system and adjust start and destination beam parameters for emitter
  (bind _returnvalue_4 (AddComponent|AddParticleSystemComponent false (Math|Transform|MakeTransform "0, 0, 0" "0.000000,0.000000,0.000000" "1.000000,1.000000,1.000000")))
  (Effects|Components|ParticleSystem|SetTemplate _returnvalue_4 ParticleSystem)
  (Transformation|AttachComponentToComponent _returnvalue_4 (Variables|Default|GetTriWayRoot) "None" "KeepRelative" "KeepRelative" "KeepRelative" true)
  (Transformation|SetRelativeLocation _returnvalue_4 (Math|Vector|MakeVector (/ (+ _x _x_2) 2.0) (/ (+ _y _y_2) 2.0) (/ (+ _z _z_2) 2.0)) false false)
  (Effects|Components|ParticleSystem|SetVectorParameter _returnvalue_4 "Beam_Source" _returnvalue_3)
  (Effects|Components|ParticleSystem|SetVectorParameter _returnvalue_4 "Beam_Target" (* _returnvalue_3 -1.0))
  (bind _returnvalue_5 (Utilities|Array|Add (Variables|Default|GetPSArray) _returnvalue_4))
  (CallFunction|EnablePS _returnvalue_5 false))

(fn SetWheelYpos
  (params (WheelId :type Integer) (Location :type Vector))
  ;[1 1 1] Set relative location for wheel specified by ID
  (Transformation|SetRelativeLocation (.WheelMeshComponent (Utilities|Struct|BreakS_TriWayData (Utilities|Array|Get(acopy) (Variables|Default|GetWheelsArray) WheelId))) Location false false))

(fn SetWheelRotation
  (params (WheelId :type Integer) (Rotator :type Rotator))
  ;[1 1 1] Set Wheel relative rotation specified by wheel ID
  (Transformation|SetRelativeRotation (.WheelMeshComponent (Utilities|Struct|BreakS_TriWayData (Utilities|Array|Get(acopy) (Variables|Default|GetWheelsArray) WheelId))) Rotator false false))

(fn EnablePS
  (params (PSIndex :type Integer) (Enable :type Boolean))
  (bind _psarray (Variables|Default|GetPSArray))
  (bind _item (Utilities|Array|Get(acopy) _psarray PSIndex))
  ;[1 1 1] Activate / Deactivate particle system specified by particle system ID
  (if Enable
    (Components|Activation|Activate _item true)
    (Development|SetHiddeninGame _item false true)
    (else
      (Components|Activation|Deactivate _item)
      (Development|SetHiddeninGame _item true true))))

(fn GetPinMesh
  (params (PinColor :type E_TriWayPinColor%20Enum))
  ;[1 1 1] Get requred pin mesh by pin color type
  (switch Utilities|FlowControl|Switch|SwitchonE_TriWayPinColor PinColor
    (:NewEnumerator0
      (LocalVariables|SetOutMesh (Variables|Default|GetMeshPinRed)))
    (:NewEnumerator1
      (LocalVariables|SetOutMesh (Variables|Default|GetMeshPinBlue)))
    (:NewEnumerator2
      (LocalVariables|SetOutMesh (Variables|Default|GetMeshPinGreen))))
  (return (LocalVariables|GetOutMesh)))