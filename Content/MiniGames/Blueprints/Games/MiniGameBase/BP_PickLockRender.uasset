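; Visual actor for the lock-picking minigame that builds the lock and exposes setters and getters for posing it.
; It spawns a centered row of base and bottom meshes between end caps, sized from mesh bounds, plus metal pin, pre-pin and spring meshes per pin.
; Setters move pins and key, returning key socket positions, and compress springs through a dynamic material morph parameter.
; When solved, pre-pins can rotate around the bottom socket to match the bottom parts.
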(event EventBeginPlay
  (|CallParentFunction)
  ;[1 1 1] Store pin size X and spring lenght by mesh size
  (Variables|Default|SetPinSizeX (* (.X (Math|Vector|BreakVector (.BoxExtent (Math|BoxSphereBounds|BreakBoxSphereBounds (StaticMesh|GetBounds (Utilities|Array|Get(acopy) (Variables|Default|GetMeshTopBaseArray))))))) 2.0))
  (Variables|Default|SetSpringLenght (* (.Z (Math|Vector|BreakVector (.BoxExtent (Math|BoxSphereBounds|BreakBoxSphereBounds (StaticMesh|GetBounds (Variables|Default|GetMeshSpring)))))) 2.0)))

(event Collision|EventActorBeginOverlap
  (params (OtherActor :type Actor%20Object%20Reference)))

(event EventTick
  (params (DeltaSeconds :type Float%20%28single-precision%29)))

(fn ConstructionScript
  (|CallParentFunction))

(fn SpawnTopBaseMeshes
  (params (PinsCount :type Integer))
  (bind _pinsizex (Variables|Default|GetPinSizeX))
  (bind _lockkey (Variables|Default|GetLockKey))
  (bind _startbase (Variables|Default|GetStartBase))
  (bind _pinsizex_2 (Variables|Default|GetPinSizeX))
  (bind _returnvalue (* PinsCount _pinsizex))
  (bind _returnvalue_2 (/ _pinsizex_2 2.0))
  (bind _returnvalue_3 (/ _pinsizex 2.0))
  (bind _relativelocation (Variables|/Script/Engine.SceneComponent|GetRelativeLocation _lockkey))
  (bind _staticmesh (Variables|/Script/Engine.StaticMeshComponent|GetStaticMesh _startbase))
  (bind _returnvalue_4 (StaticMesh|GetBounds _staticmesh))
  (bind _returnvalue_5 (/ _returnvalue -2.0))
  (bind (_x _y _z) (Math|Vector|BreakVector _relativelocation))
  (bind _boxextent (Math|BoxSphereBounds|BreakBoxSphereBounds _returnvalue_4))
  (bind _returnvalue_6 (+ _returnvalue_5 _returnvalue_3))
  (bind _x_2 (Math|Vector|BreakVector _boxextent))
  (bind _returnvalue_7 (* _x_2 0.985))
  ;[1 1 1] Spawn requred by count of top base (wood) meshes and start-finish decor meshes
  (Utilities|Array|Clear (Variables|Default|GetMeshBottomArray))
  (Variables|Default|SetStartXPosition _returnvalue_6)
  (LocalVariables|SetTempPosition _returnvalue_6)
  (for _index (range 0 (- PinsCount 1))
    (bind _returnvalue_8 (AddComponent|AddStaticMeshComponent false (Math|Transform|MakeTransform (Math|Vector|MakeVector (LocalVariables|GetTempPosition) 0.0 0.0) "0,0.000000, 0")))
    (Components|StaticMesh|SetStaticMesh _returnvalue_8 (Utilities|Array|Get(acopy) (Variables|Default|GetMeshTopBaseArray) _index))
    (bind _output_get (LocalVariables|SetMeshComponent _returnvalue_8))
    (if (== _index 0)
      (Variables|Default|SetBottomSocketLocation (.Location (Math|Transform|BreakTransform (Transformation|GetSocketTransform (LocalVariables|GetMeshComponent) "BottomCenter" "RTS_Component")))))
    (Transformation|AttachComponentToComponent _output_get (Variables|Default|GetPickLockRoot) "None" "KeepRelative" "KeepRelative" "KeepRelative" true)
    (bind _returnvalue_9 (AddComponent|AddStaticMeshComponent false (Math|Transform|MakeTransform (Math|Vector|MakeVector (LocalVariables|GetTempPosition) (.Y (Math|Vector|BreakVector (Variables|Default|GetBottomSocketLocation))) (.Z (Math|Vector|BreakVector (Variables|Default|GetBottomSocketLocation)))) "0,0.000000, 0")))
    (Components|StaticMesh|SetStaticMesh _returnvalue_9 (Variables|Default|GetMeshBottom))
    (Transformation|AttachComponentToComponent _returnvalue_9 (Variables|Default|GetPickLockRoot) "None" "KeepRelative" "KeepRelative" "KeepRelative" true)
    (Utilities|Array|Add (Variables|Default|GetMeshBottomArray) _returnvalue_9)
    (LocalVariables|SetTempPosition (+ (LocalVariables|GetTempPosition) (Variables|Default|GetPinSizeX))))
  (Variables|Default|SetKeyInitLocation (Math|Vector|MakeVector (Variables|Default|GetStartXPosition) _y _z))
  (Variables|Default|SetBPointInitLocation (+ (Variables|/Script/Engine.SceneComponent|GetRelativeLocation (Variables|Default|GetBpoint)) (Math|Vector|MakeVector (Variables|Default|GetStartXPosition) 0.0 0.0)))
  (Variables|Default|SetBSegmentLenght (Math|Vector|VectorLength (- (Math|Vector|MakeVector (Variables|Default|GetStartXPosition) _y _z) (+ (Variables|/Script/Engine.SceneComponent|GetRelativeLocation (Variables|Default|GetBpoint)) (Math|Vector|MakeVector (Variables|Default|GetStartXPosition) 0.0 0.0)))))
  (Transformation|SetRelativeLocation _startbase (Math|Vector|MakeVector (- (Variables|Default|GetStartXPosition) (+ _returnvalue_2 _returnvalue_7)) 0.0 0.0) false false)
  (Transformation|SetRelativeLocation (Variables|Default|GetEndBase) (Math|Vector|MakeVector (- (+ (LocalVariables|GetTempPosition) _returnvalue_7) _returnvalue_2) 0.0 0.0) false false))

(fn SetKeyLocation
  (params (Xposition :type Float%20%28single-precision%29) (Angle :type Float%20%28single-precision%29))
  (bind _returnvalue (Math|Vector|MakeVector Xposition 0.0 0.0))
  (bind _picklockroot (Variables|Default|GetPickLockRoot))
  (bind _keyinitlocation (Variables|Default|GetKeyInitLocation))
  (bind _lockkey (Variables|Default|GetLockKey))
  (bind _lockkey_2 (Variables|Default|GetLockKey))
  (bind _returnvalue_2 (Transformation|GetWorldTransform _picklockroot))
  (bind _returnvalue_3 (+ _returnvalue _keyinitlocation))
  ;[1 1 1] Set Key relative location and get actual locations from sockets - Start, End. Socked defined in the Key mesh
  (Transformation|SetRelativeLocation _lockkey _returnvalue_3 false false)
  (Transformation|SetRelativeRotation _lockkey (Math|Rotator|MakeRotator 0.0 Angle 0.0) false false)
  (return (Math|Transform|InverseTransformLocation _returnvalue_2 (Transformation|GetSocketLocation _lockkey_2 "KeyStart")) (Math|Transform|InverseTransformLocation _returnvalue_2 (Transformation|GetSocketLocation _lockkey_2 "KeyEnd")) _returnvalue_3))

(fn GetKeyInitLocation
  ;[1 1 1] Helper function. Get initial Key location
  (return (Variables|Default|GetKeyInitLocation)))

(fn GetPinSize
  ;[1 1 1] Return pin X size
  (return (Variables|Default|GetPinSizeX)))

(fn GetLPointLocation
  ;[1 1 1] Get L (need for Key) point relative location
  (return (Variables|/Script/Engine.SceneComponent|GetRelativeLocation (Variables|Default|GetLPoint))))

(fn GetBPointLocation
  ;[1 1 1] Get B (need for Key) point initial location
  (return (Variables|Default|GetBPointInitLocation)))

(fn SpawnPin
  (params (PinData :type S%20Pick%20Lock%20Pin%20Data%20Structure))
  (bind (_metalpinstate _prepinstate _pinlenght _metalpincounter _metalpinzpos _metalpinzoffset _prepincounter _prepinzpos _xpos _prepinzoffset _springzpos) (Utilities|Struct|BreakS_PickLockPinData PinData))
  (bind _bottomsocketlocation (Variables|Default|GetBottomSocketLocation))
  (bind _y (Math|Vector|BreakVector _bottomsocketlocation))
  (bind _returnvalue (+ _metalpinzpos _metalpinzoffset))
  (bind _returnvalue_2 (+ _prepinzoffset _prepinzpos))
  (bind _returnvalue_3 (Math|Vector|MakeVector _xpos _y _returnvalue_2))
  (bind _returnvalue_4 (Math|Vector|MakeVector _xpos _y _returnvalue))
  ;[1 1 1] Spawn Metal pin, Pre pin and Spring meshes by pin data structure. Create and set dynamic material for spring mesh
  (bind (_meshmetalpin _meshprepin) (CallFunction|GetMeshesbyPinLenght _pinlenght))
  (bind _returnvalue_5 (AddComponent|AddStaticMeshComponent false (Math|Transform|MakeTransform _returnvalue_4 "0,0.000000,0.000000" "1,1,1.000000")))
  (Components|StaticMesh|SetStaticMesh _returnvalue_5 _meshmetalpin)
  (Transformation|AttachComponentToComponent _returnvalue_5 (Variables|Default|GetPickLockRoot) "None" "KeepRelative" "KeepRelative" "KeepRelative" true)
  (bind _returnvalue_6 (AddComponent|AddStaticMeshComponent false (Math|Transform|MakeTransform _returnvalue_3 "0,0.000000, 0")))
  (Components|StaticMesh|SetStaticMesh _returnvalue_6 _meshprepin)
  (Transformation|AttachComponentToComponent _returnvalue_6 (Variables|Default|GetPickLockRoot) "None" "KeepRelative" "KeepRelative" "KeepRelative" true)
  (bind _returnvalue_7 (AddComponent|AddStaticMeshComponent false (Math|Transform|MakeTransform (Math|Vector|MakeVector _xpos (Variables|Default|GetSpringYOffset) _springzpos) "0,0.000000,0.000000" "1.000000,1.000000,1.000000")))
  (Components|StaticMesh|SetStaticMesh _returnvalue_7 (Variables|Default|GetMeshSpring))
  (Transformation|AttachComponentToComponent _returnvalue_7 (Variables|Default|GetPickLockRoot) "None" "KeepRelative" "KeepRelative" "KeepRelative" true)
  (bind _returnvalue_8 (Rendering|Material|CreateDynamicMaterialInstance "/Game/MiniGames/Materials/PickLock/M_PickLockSpring.M_PickLockSpring" :!class /Script/Engine.KismetMaterialLibrary))
  (Rendering|Material|SetMaterial _returnvalue_7 0 _returnvalue_8)
  (Utilities|Array|Add (Variables|Default|GetMeshPinsArray) (Utilities|Struct|MakeS_PickLockPin _returnvalue_4 _returnvalue_3 _returnvalue_5 _returnvalue_6 _returnvalue_7 _returnvalue_8)))

(fn SetPrePinParameters
  (params (PinIndex :type Integer) (PrePinZPos :type Float%20%28single-precision%29) (PrePinZOffset :type Float%20%28single-precision%29))
  (bind _returnvalue (+ PrePinZPos PrePinZOffset))
  (bind _meshpinsarray (Variables|Default|GetMeshPinsArray))
  (bind _item (Utilities|Array|Get(acopy) _meshpinsarray PinIndex))
  (bind (_metalpinlocation _prepinlocation _meshmetalpin _meshprepin _meshspring _springmaterial) (Utilities|Struct|BreakS_PickLockPin _item))
  (bind (_x _y) (Math|Vector|BreakVector _prepinlocation))
  (bind _returnvalue_2 (Math|Vector|MakeVector _x _y _returnvalue))
  ;[1 1 1] Set Pre pin dynamic parameters by Pre pin Index
  (Transformation|SetRelativeLocation _meshprepin _returnvalue_2 false false)
  (Utilities|Array|SetArrayElem _meshpinsarray PinIndex (Utilities|Struct|MakeS_PickLockPin _metalpinlocation _returnvalue_2 _meshmetalpin _meshprepin _meshspring _springmaterial)))

(fn GetBSegLenght
  ;[1 1 1] Return B segment lenght. Need for Key calculation
  (return (Variables|Default|GetBSegmentLenght)))

(fn GetStartXPosition
  ;[1 1 1] Helper. Get Start spawn X position
  (return (Variables|Default|GetStartXPosition)))

(fn GetPinsLenght
  ;[1 1 1] Get metal pins, pre pins and spring lenght by type
  (return (* (.Z (Math|Vector|BreakVector (.BoxExtent (Math|BoxSphereBounds|BreakBoxSphereBounds (StaticMesh|GetBounds (Variables|Default|GetMeshMetalPinLong)))))) 2.0) (* (.Z (Math|Vector|BreakVector (.BoxExtent (Math|BoxSphereBounds|BreakBoxSphereBounds (StaticMesh|GetBounds (Variables|Default|GetMeshMetalPinMiddle)))))) 2.0) (* (.Z (Math|Vector|BreakVector (.BoxExtent (Math|BoxSphereBounds|BreakBoxSphereBounds (StaticMesh|GetBounds (Variables|Default|GetMeshMetalPinShort)))))) 2.0) (* (.Z (Math|Vector|BreakVector (.BoxExtent (Math|BoxSphereBounds|BreakBoxSphereBounds (StaticMesh|GetBounds (Variables|Default|GetMeshPrePinLong)))))) 2.0) (* (.Z (Math|Vector|BreakVector (.BoxExtent (Math|BoxSphereBounds|BreakBoxSphereBounds (StaticMesh|GetBounds (Variables|Default|GetMeshPrePinMiddle)))))) 2.0) (* (.Z (Math|Vector|BreakVector (.BoxExtent (Math|BoxSphereBounds|BreakBoxSphereBounds (StaticMesh|GetBounds (Variables|Default|GetMeshPrePinShort)))))) 2.0) (* (.Z (Math|Vector|BreakVector (.BoxExtent (Math|BoxSphereBounds|BreakBoxSphereBounds (StaticMesh|GetBounds (Variables|Default|GetMeshSpring)))))) 2.0)))

(fn GetMeshesbyPinLenght
  (params (PinLenght :type E_PickLockPinLen%20Enum))
  ;[1 1 1] Get requred mesh by specified pin length
  (switch Utilities|FlowControl|Switch|SwitchonE_PickLockPinLen PinLenght
    (:NewEnumerator0
      (LocalVariables|SetMetalMesh (Variables|Default|GetMeshMetalPinShort))
      (LocalVariables|SetPreMesh (Variables|Default|GetMeshPrePinLong)))
    (:NewEnumerator1
      (LocalVariables|SetMetalMesh (Variables|Default|GetMeshMetalPinMiddle))
      (LocalVariables|SetPreMesh (Variables|Default|GetMeshPrePinMiddle)))
    (:NewEnumerator2
      (LocalVariables|SetMetalMesh (Variables|Default|GetMeshMetalPinLong))
      (LocalVariables|SetPreMesh (Variables|Default|GetMeshPrePinShort))))
  (return (LocalVariables|GetMetalMesh) (LocalVariables|GetPreMesh)))

(fn GetPrePinLocation
  (params (Index :type Integer))
  ;[1 1 1] Get Pre pin relative location
  (return (.PrePinLocation (Utilities|Struct|BreakS_PickLockPin (Utilities|Array|Get(acopy) (Variables|Default|GetMeshPinsArray) Index)))))

(fn SetMetalPinParameters
  (params (PinIndex :type Integer) (MetalPinZpos :type Float%20%28single-precision%29) (MetalPinZOffset :type Float%20%28single-precision%29))
  (bind _meshpinsarray (Variables|Default|GetMeshPinsArray))
  (bind _item (Utilities|Array|Get(acopy) _meshpinsarray PinIndex))
  (bind (_metalpinlocation _prepinlocation _meshmetalpin) (Utilities|Struct|BreakS_PickLockPin _item))
  (bind (_x _y) (Math|Vector|BreakVector _metalpinlocation))
  ;[1 1 1] Set Metal pin dynamic parameters by index
  (Transformation|SetRelativeLocation _meshmetalpin (Math|Vector|MakeVector _x _y (+ MetalPinZpos MetalPinZOffset)) false false))

(fn SetSpringParameters
  (params (PinIndex :type Integer) (Scale :type Float%20%28single-precision%29))
  ;[1 1 1] Pass morphing (scale) parameter to spring mesh material
  (Rendering|Material|SetScalarParameterValue (.SpringMaterial (Utilities|Struct|BreakS_PickLockPin (Utilities|Array|Get(acopy) (Variables|Default|GetMeshPinsArray) PinIndex))) "SpringMorph" (Math|Float|Clamp(Float) (- 1.0 Scale)) :!class /Script/Engine.MaterialInstanceDynamic))

(fn SetBottomParameters
  (params (Angle :type Float%20%28single-precision%29))
  (bind _meshbottomarray (Variables|Default|GetMeshBottomArray))
  ;[1 1 1] Set parameter (rotation) for all spawned bottom mettal parts
  (for (_ _array_index) _meshbottomarray
    (Transformation|SetRelativeRotation (Utilities|Array|Get(acopy) _meshbottomarray _array_index) (Math|Rotator|MakeRotator Angle 0.0 0.0) false false)))

(fn SetPrePinsRotation
  (params (Angle :type Float%20%28single-precision%29))
  (bind _returnvalue (Math|Rotator|MakeRotator Angle 0.0 0.0))
  (bind _bottomsocketlocation (Variables|Default|GetBottomSocketLocation))
  (bind (_x _y _z) (Math|Vector|BreakVector _bottomsocketlocation))
  ;[1 1 1] Calculate actual rotation for pre pins when lock is solved. Rotation are same with bottom parts
  (for _array_element (Variables|Default|GetMeshPinsArray)
    (Transformation|SetRelativeLocationAndRotation (.MeshPrePin (Utilities|Struct|BreakS_PickLockPin _array_element)) (+ (Math|Vector|MakeVector (.X (Math|Vector|BreakVector (.PrePinLocation (Utilities|Struct|BreakS_PickLockPin _array_element)))) (.Y (Math|Vector|BreakVector (Math|Vector|RotateVector (Math|Vector|MakeVector 0.0 0.0 (- (Math|Float|Absolute(Float) _z) (Math|Float|Absolute(Float) (.Z (Math|Vector|BreakVector (.PrePinLocation (Utilities|Struct|BreakS_PickLockPin _array_element))))))) _returnvalue))) (.Z (Math|Vector|BreakVector (Math|Vector|RotateVector (Math|Vector|MakeVector 0.0 0.0 (- (Math|Float|Absolute(Float) _z) (Math|Float|Absolute(Float) (.Z (Math|Vector|BreakVector (.PrePinLocation (Utilities|Struct|BreakS_PickLockPin _array_element))))))) _returnvalue)))) (Math|Vector|MakeVector 0.0 _y _z)) _returnvalue false false)))

(fn SetRootXPos
  (params (Xpos :type Float%20%28single-precision%29))
  (bind _picklockroot (Variables|Default|GetPickLockRoot))
  ;[1 1 1] Helper function. Set PickLock root relative location
  (Transformation|SetRelativeLocation _picklockroot (+ (Math|Vector|MakeVector 0.0 Xpos 0.0) (Variables|/Script/Engine.SceneComponent|GetRelativeLocation _picklockroot)) false false))