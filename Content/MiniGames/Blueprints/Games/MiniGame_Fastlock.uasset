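; FastLock minigame Blueprint where the player rotates a ring of segments to match a randomized finish segment.
; It spawns BP_FastLockRender for visuals, shuffles segment order and accepts up, down and select inputs.
; A Tick state machine animates meshes, shifting the order array and resetting root rotation after each 22.5-degree step.
; Selection thrusts the start segment forward; matches increase completion and reroll the finish segment, while misses decrease completion.
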(event EventBeginPlay
  (|CallParentFunction)
  ;[1 1 1] Setup initial variables and rotation speed
  (Variables|Default|SetOffsetSpeed (* (/ (Variables|Default|GetStartSegmentMaxOffset) (Math|Float|MakeLiteralFloat 22.5)) (Variables|GameFastLock|GetRotationSpeed)))
  (Variables|Default|SetToggleOffsetMax 4.21)
  (Variables|Default|SetFinishOffsetMax 1e+01))

(event EventTick
  (params (DeltaSeconds :type Float%20%28single-precision%29))
  (bind _togglespeed (Variables|GameFastLock|GetToggleSpeed))
  (bind _fastlockrender (Variables|Default|GetFastLockRender))
  (bind _fastlockrender_2 (Variables|Default|GetFastLockRender))
  (bind _finishoffsetmax (Variables|Default|GetFinishOffsetMax))
  (bind _finishoffsetmax_2 (Variables|Default|GetFinishOffsetMax))
  (bind _returnvalue (* DeltaSeconds _togglespeed))
  ;[1 1 1] State machine
  (|CallParentFunction DeltaSeconds)
  (bind _iswantexit (CallFunction|GetWantExit))
  (if _iswantexit
    ;;[1 1 1] Set game ready to exit
    (Variables|Default|SetFastLockState "NewEnumerator3")
    (CallFunction|SetProcesstoExit true)
    (else
      (switch Utilities|FlowControl|Switch|SwitchonE_MiniGameState (CallFunction|GetMiniGameState)
        (:NewEnumerator1
          (switch Utilities|FlowControl|Switch|SwitchonE_FastLockState (Variables|Default|GetFastLockState)
            (:NewEnumerator0
              ;;[1 1 1] Rotate Up / Down segmetns
              (Variables|Default|SetDirectionRotUp true)
              (bind _output_get (Variables|Default|SetRotationAngle (Math|Float|Clamp(Float) (+ (Variables|Default|GetRotationAngle) (* DeltaSeconds (Variables|GameFastLock|GetRotationSpeed))) 0.0 22.5) :!label _label))
              (if (>= _output_get 22.5)
                (Variables|Default|SetFastLockState "NewEnumerator6")
                (CallFunction|ShiftSegmentsArray (Variables|Default|GetDirectionRotUp))
                (Default|RotateRoot _fastlockrender 0.0)
                (CallFunction|UpdateSegmentsMeshes)
                (Default|SetMeshOffset _fastlockrender 0 (Variables|Default|GetStartSegmentMaxOffset))
                (Variables|Default|SetRotationAngle 0.0)
                (Variables|Default|SetSegmentOffsetCounter 0.0)
                (if (Variables|Default|GetDirectionRotUp)
                  (Default|SetMeshOffset _fastlockrender 2 0.0)
                  (else
                    (Default|SetMeshOffset _fastlockrender 1 0.0)))
                (else
                  (Default|SetMeshOffset _fastlockrender 0 (- (Variables|Default|GetStartSegmentMaxOffset) (Variables|Default|GetSegmentOffsetCounter)))
                  (if (Variables|Default|GetDirectionRotUp)
                    (Default|SetMeshOffset _fastlockrender 2 (Variables|Default|GetSegmentOffsetCounter))
                    (Default|RotateRoot _fastlockrender (Variables|Default|GetRotationAngle))
                    (else
                      (Default|SetMeshOffset _fastlockrender 1 (Variables|Default|GetSegmentOffsetCounter))
                      (Default|RotateRoot _fastlockrender (* (Variables|Default|GetRotationAngle) -1.0))))
                  (Variables|Default|SetSegmentOffsetCounter (Math|Float|Clamp(Float) (+ (Variables|Default|GetSegmentOffsetCounter) (* DeltaSeconds (Variables|Default|GetOffsetSpeed))) 0.0 (Variables|Default|GetStartSegmentMaxOffset))))))
            (:NewEnumerator1
              (Variables|Default|SetDirectionRotUp false)
              (goto _label))
            (:NewEnumerator2
              ;;[0 0.9767 1] Select
              (CallFunction|CheckSegmentsEquality)
              (Variables|Default|SetFastLockState "NewEnumerator5"))
            (:NewEnumerator5
              ;;[1 1 1] Move start segment to finish. Play sound on finish
              (Default|SetMeshOffset (Variables|Default|GetFastLockRender) 0 (+ (Variables|Default|GetStartSegmentMaxOffset) (Variables|Default|GetSegmentOffsetCounter)))
              (bind _output_get_2 (Variables|Default|SetSegmentOffsetCounter (Math|Float|Clamp(Float) (+ (Variables|Default|GetSegmentOffsetCounter) _returnvalue) 0.0 (Variables|Default|GetToggleOffset))))
              (if (>= _output_get_2 (Variables|Default|GetToggleOffset))
                (Variables|Default|SetSegmentOffsetCounter 0.0)
                (Variables|Default|SetFastLockState "NewEnumerator4")
                (Variables|Default|SetFinishOffsetCounter 0.0)
                (Variables|Default|SetGetBackFinishSegment false)
                (Variables|Default|SetIsStartSegmentComplete false)
                (Variables|Default|SetIsFinishSegmentComplete false)
                (if (Variables|Default|GetIsStartEqualFinish)
                  (CallFunction|PlaySoundCue (Variables|Sounds|GetMatched) 0.0)
                  (else
                    (CallFunction|PlaySoundCue (Variables|Sounds|GetNotMatch) 0.0)
                    (CallFunction|DecreaseComplete)))))
            (:NewEnumerator4
              (Utilities|FlowControl|Sequence
                (:then_0
                  ;;[1 1 1] Move start segments to init location and randomize finish segments if requred
                  (Default|SetMeshOffset (Variables|Default|GetFastLockRender) 0 (- (+ (Variables|Default|GetStartSegmentMaxOffset) (Variables|Default|GetToggleOffset)) (Variables|Default|GetSegmentOffsetCounter)))
                  (bind _output_get_3 (Variables|Default|SetSegmentOffsetCounter (Math|Float|Clamp(Float) (+ (Variables|Default|GetSegmentOffsetCounter) _returnvalue) 0.0 (Variables|Default|GetToggleOffset))))
                  (if (>= _output_get_3 (Variables|Default|GetToggleOffset))
                    (Variables|Default|SetIsStartSegmentComplete true)))
                (:then_1
                  (if (Variables|Default|GetIsStartEqualFinish)
                    (if (Variables|Default|GetGetBackFinishSegment)
                      (Default|SetMeshOffset _fastlockrender_2 3 (- (Variables|Default|GetFinishOffsetMax) (+ (Variables|Default|GetFinishOffsetCounter) _returnvalue)))
                      (Variables|Default|SetFinishOffsetCounter (Math|Float|Clamp(Float) (+ (Variables|Default|GetFinishOffsetCounter) _returnvalue) 0.0 _finishoffsetmax))
                      (if (>= (Math|Float|Clamp(Float) (+ (Variables|Default|GetFinishOffsetCounter) _returnvalue) 0.0 _finishoffsetmax) _finishoffsetmax)
                        (Variables|Default|SetIsFinishSegmentComplete true))
                      (else
                        (Default|SetMeshOffset _fastlockrender_2 3 (+ (Variables|Default|GetFinishOffsetCounter) _returnvalue))
                        (Variables|Default|SetFinishOffsetCounter (Math|Float|Clamp(Float) (+ (Variables|Default|GetFinishOffsetCounter) _returnvalue) 0.0 _finishoffsetmax_2))
                        (if (>= (Math|Float|Clamp(Float) (+ (Variables|Default|GetFinishOffsetCounter) _returnvalue) 0.0 _finishoffsetmax_2) _finishoffsetmax_2)
                          (Variables|Default|SetGetBackFinishSegment true)
                          (CallFunction|RandomizeFinishSegment)
                          (CallFunction|UpdateFinishMesh)
                          (Variables|Default|SetFinishOffsetCounter 0.0))))
                    (else
                      (Variables|Default|SetIsFinishSegmentComplete true))))
                (:then_2
                  ;;[0 0.9767 1] Swith to Play state when all segments are ready
                  (if (not (not (and (Variables|Default|GetIsStartSegmentComplete) (Variables|Default|GetIsFinishSegmentComplete))))
                    (Variables|Default|SetFinishOffsetCounter 0.0)
                    (Variables|Default|SetSegmentOffsetCounter 0.0)
                    (if (Variables|Default|GetIsStartEqualFinish)
                      (CallFunction|IncreaseComplete))
                    (Variables|Default|SetFastLockState "NewEnumerator6")))))))))))

(event EventSpawnMiniGame
  ;[1 1 1] Spawn FastLock render and adjust ingame variables. Randomize segments
  (Variables|Default|SetRotationAngle 0.0)
  (Variables|Default|SetSegmentOffsetCounter 0.0)
  (bind (_transfrom _isvalid) (CallFunction|GetAnchorTransform))
  (if _isvalid
    (bind _returnvalue (Game|SpawnActorfromClass "/Game/MiniGames/Blueprints/Games/MiniGameBase/BP_FastLockRender.BP_FastLockRender_C" _transfrom "Undefined" 0 0))
    (Utilities|IsValid _returnvalue
      (:Is%20Valid
        (CallFunction|SetRenderPtr _returnvalue)
        (bind _output_get (Variables|Default|SetFastLockRender _returnvalue))
        (bind (_lenght _location) (Default|GetStartSegLengthLocation _output_get))
        (Variables|Default|SetStartSegLenght _lenght)
        (Variables|Default|SetStartSegLocation _location)
        (bind _newparam (Default|GetFinishSegLocation _output_get))
        (Variables|Default|SetFinishSegLocation _newparam)
        (CallFunction|RandomizeSegments)
        (CallFunction|UpdateSegmentsMeshes)
        (Default|SetMeshOffset _output_get 0 (Variables|Default|GetStartSegmentMaxOffset))
        (CallFunction|CheckSegmentsEquality)
        (Variables|Default|SetFastLockState "NewEnumerator6")
        (CallFunction|SetNeedtoComplete (Variables|GameFastLock|GetCompleteCount))
        (CallFunction|SetGameSpawned true))
      (:Is%20Not%20Valid
        (Development|PrintString "Error: FastLock -> Cant spawn BP_Render" true true "(R=1.000000,G=0.000000,B=0.000000,A=1.000000)" 5.0)))))

(event EventTogglePressed
  ;[1 1 1] Steering events. Check UP / Down / Select actions
  (if (and (Utilities|Enum|Equal(Enum) (Variables|Default|GetFastLockState) "NewEnumerator6") (Utilities|Enum|Equal(Enum) (CallFunction|GetMiniGameState) "NewEnumerator1"))
    (Variables|Default|SetFastLockState "NewEnumerator2")))

(event EventUpPressed
  ;[1 1 1] Steering events. Check UP / Down / Select actions
  (if (and (Utilities|Enum|Equal(Enum) (Variables|Default|GetFastLockState) "NewEnumerator6") (Utilities|Enum|Equal(Enum) (CallFunction|GetMiniGameState) "NewEnumerator1"))
    (Variables|Default|SetFastLockState "NewEnumerator0")))

(event EventDownPressed
  ;[1 1 1] Steering events. Check UP / Down / Select actions
  (if (and (Utilities|Enum|Equal(Enum) (Variables|Default|GetFastLockState) "NewEnumerator6") (Utilities|Enum|Equal(Enum) (CallFunction|GetMiniGameState) "NewEnumerator1"))
    (Variables|Default|SetFastLockState "NewEnumerator1")))

(fn RandomizeSegments
  (bind _lastindex (Variables|Default|GetLastIndex))
  (bind _segmentsorder (Variables|Default|GetSegmentsOrder))
  ;[1 1 1] Create and mix game segments order in the array
  (Utilities|Array|Clear (Variables|Default|GetSegmentsOrder))
  (for _index (range 0 _lastindex)
    (Utilities|Array|SetArrayElem (Variables|Default|GetSegmentsOrder) _index _index true))
  (for _index_2 (range 0 (Variables|Default|GetLastIndex))
    (bind _output_get (LocalVariables|SetIndex1 (Math|Random|RandomIntegerinRange 0 _lastindex)))
    (LocalVariables|SetValue1 (Utilities|Array|Get(acopy) _segmentsorder _output_get))
    (bind _output_get_2 (LocalVariables|SetIndex2 (Math|Random|RandomIntegerinRange 0 _lastindex)))
    (LocalVariables|SetValue2 (Utilities|Array|Get(acopy) _segmentsorder _output_get_2))
    (Utilities|Array|SetArrayElem (Variables|Default|GetSegmentsOrder) (LocalVariables|GetIndex1) (LocalVariables|GetValue2) true)
    (Utilities|Array|SetArrayElem (Variables|Default|GetSegmentsOrder) (LocalVariables|GetIndex2) (LocalVariables|GetValue1) true))
  (CallFunction|RandomizeFinishSegment))

(fn ShiftSegmentsArray
  (params (ShiftUp :type Boolean))
  (bind _segmentsorder (Variables|Default|GetSegmentsOrder))
  (bind _segmentsorder_2 (Variables|Default|GetSegmentsOrder))
  (bind _segmentsorder_3 (Variables|Default|GetSegmentsOrder))
  (bind _lastindex (Variables|Default|GetLastIndex))
  ;[1 1 1] Sift Up / Down segments array specified by direction
  (if ShiftUp
    (LocalVariables|SetFirstIndexValue (Utilities|Array|Get(acopy) _segmentsorder_3 _lastindex))
    (for _index (range 1 _lastindex)
      (Utilities|Array|SetArrayElem _segmentsorder_2 (+ (- _lastindex _index) 1) (Utilities|Array|Get(acopy) _segmentsorder_2 (- _lastindex _index))))
    (Utilities|Array|SetArrayElem (Variables|Default|GetSegmentsOrder) 0 (LocalVariables|GetFirstIndexValue))
    (else
      (LocalVariables|SetFirstIndexValue (Utilities|Array|Get(acopy) _segmentsorder_3))
      (for _index_2 (range 1 (Variables|Default|GetLastIndex))
        (Utilities|Array|SetArrayElem _segmentsorder (- _index_2 1) (Utilities|Array|Get(acopy) _segmentsorder _index_2)))
      (Utilities|Array|SetArrayElem (Variables|Default|GetSegmentsOrder) (Variables|Default|GetLastIndex) (LocalVariables|GetFirstIndexValue)))))

(fn UpdateSegmentsMeshes
  ;[1 1 1] Update actual meshes in the render specified by segments array mesh indices
  (for _index (range 0 (Variables|Default|GetLastIndex))
    (Default|SetSegmentMesh (Variables|Default|GetFastLockRender) _index (.Start (Utilities|Struct|BreakS_FastLockSegment (Utilities|Array|Get(acopy) (Variables|Default|GetStartFinishSegmentsMeshes) (Utilities|Array|Get(acopy) (Variables|Default|GetSegmentsOrder) _index))))))
  (CallFunction|UpdateFinishMesh))

(fn RandomizeFinishSegment
  ;[1 1 1] Set random finish segment index
  (Variables|Default|SetFinishSegmentIndex (Math|Random|RandomIntegerinRange 0 (Variables|Default|GetLastIndex))))

(fn UpdateFinishMesh
  ;[1 1 1] Update current finish mesh segment
  (Default|SetFinishSegmentMesh (Variables|Default|GetFastLockRender) (.Finish (Utilities|Struct|BreakS_FastLockSegment (Utilities|Array|Get(acopy) (Variables|Default|GetStartFinishSegmentsMeshes) (Variables|Default|GetFinishSegmentIndex))))))

(fn CheckSegmentsEquality
  (bind _finishseglocation (Variables|Default|GetFinishSegLocation))
  (bind _startseglocation (Variables|Default|GetStartSegLocation))
  (bind _startseglenght (Variables|Default|GetStartSegLenght))
  (bind _startsegmentmaxoffset (Variables|Default|GetStartSegmentMaxOffset))
  (bind _returnvalue (- _finishseglocation _startseglocation))
  (bind _returnvalue_2 (+ _startseglenght _startsegmentmaxoffset))
  (bind _returnvalue_3 (Math|Vector|VectorLength _returnvalue))
  (bind _returnvalue_4 (- _returnvalue_3 _returnvalue_2))
  ;[1 1 1] Check start and finish segments equality. Calculate actual toggle offset value
  (bind _output_get (Variables|Default|SetIsStartEqualFinish (== (Utilities|Array|Get(acopy) (Variables|Default|GetSegmentsOrder)) (Variables|Default|GetFinishSegmentIndex))))
  (if _output_get
    (Variables|Default|SetToggleOffset (+ _returnvalue_4 (Variables|Default|GetToggleOffsetMax)))
    (else
      (Variables|Default|SetToggleOffset _returnvalue_4))))