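; Radar minigame where the player presses toggle while a rotating ray covers a good point to build up the completion count.
; Spawns a BP_RadarRender and drives ray, point and flash through a dynamic M_RadarRay material.
; Tick rotates the ray, runs the Play/Good/Bad state machine and re-places the random good or bad point once swept.
; Hit testing compares the point's angle to the ray's arc; bad hits and misses decrease completion.
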(event EventBeginPlay
  (|CallParentFunction))

(event EventTick
  (params (DeltaSeconds :type Float%20%28single-precision%29))
  (bind _flashcolorcurve (Variables|Default|GetFlashColorCurve))
  (bind _flashcolorcurve_2 (Variables|Default|GetFlashColorCurve))
  ;[1 1 1] State machine
  (|CallParentFunction DeltaSeconds)
  (bind _iswantexit (CallFunction|GetWantExit))
  (if _iswantexit
    ;;[1 1 1] Game ready to exit
    (Variables|Default|SetRadarState "NewEnumerator0")
    (CallFunction|SetProcesstoExit true)
    (else
      (bind _gamespawned (CallFunction|GetGameSpawned))
      (if _gamespawned
        (CallFunction|RotateRay DeltaSeconds)
        (switch Utilities|FlowControl|Switch|SwitchonE_RadarState (Variables|Default|GetRadarState)
          (:NewEnumerator5
            ;;[1 1 1] If ray leave current point then place new one
            (bind _ispointunderray (CallFunction|CheckPoint))
            (if (and (not (Variables|Default|GetPointUnderRay)) _ispointunderray)
              (Variables|Default|SetPointUnderRay true)
              (elif (and (Variables|Default|GetPointUnderRay) (not _ispointunderray))
                (CallFunction|PlacePoint))))
          (:NewEnumerator2
            ;;[1 1 1] Bad point effect
            (bind _output_get (Variables|Default|SetPostColorCounter (+ (Variables|Default|GetPostColorCounter) (* DeltaSeconds (Variables|GameRadar|GetFlashColorSpeed)))))
            (CallFunction|SetPostColor (Variables|GameRadar|GetFlashBadColor) (Math|Curves|GetFloatValue _flashcolorcurve_2 _output_get))
            (if (>= (+ (Variables|Default|GetPostColorCounter) (* DeltaSeconds (Variables|GameRadar|GetFlashColorSpeed))) (.MaxTime (Math|Curves|GetTimeRange _flashcolorcurve_2)))
              (Variables|Default|SetRadarState "NewEnumerator5")))
          (:NewEnumerator3
            ;;[1 1 1] Good point effect
            (bind _output_get_2 (Variables|Default|SetPostColorCounter (+ (Variables|Default|GetPostColorCounter) (* DeltaSeconds (Variables|GameRadar|GetFlashColorSpeed)))))
            (CallFunction|SetPostColor (Variables|GameRadar|GetFlashGoodColor) (Math|Curves|GetFloatValue _flashcolorcurve _output_get_2))
            (if (>= (+ (Variables|Default|GetPostColorCounter) (* DeltaSeconds (Variables|GameRadar|GetFlashColorSpeed))) (.MaxTime (Math|Curves|GetTimeRange _flashcolorcurve)))
              (Variables|Default|SetRadarState "NewEnumerator5"))))))))

(event EventSpawnMiniGame
  ;[1 1 1] Spawn Radar  render and setup variables
  (bind (_transfrom _isvalid) (CallFunction|GetAnchorTransform))
  (if _isvalid
    (bind _returnvalue (Game|SpawnActorfromClass "/Game/MiniGames/Blueprints/Games/MiniGameBase/BP_RadarRender.BP_RadarRender_C" _transfrom "Undefined" 0 0))
    (Utilities|IsValid _returnvalue
      (:Is%20Valid
        (CallFunction|SetRenderPtr _returnvalue)
        (bind _output_get (Variables|Default|SetRadarRender _returnvalue))
        (bind _material (CallFunction|CreateDynamicMaterial))
        (Default|SetRadarMaterial _output_get _material)
        (Variables|Default|SetRayCounter (Math|Random|RandomFloatinRange 0.0 0.75))
        (CallFunction|SetRayFocus (Variables|GameRadar|GetFocusSize))
        (Rendering|Material|SetVectorParameterValue (Variables|Default|GetRadarRayMaterial) "RayColor" (Variables|GameRadar|GetRayColor) :!class /Script/Engine.MaterialInstanceDynamic)
        (CallFunction|PlacePoint)
        (CallFunction|SetNeedtoComplete (Variables|GameRadar|GetCompleteCount))
        (Variables|Default|SetRadarState "NewEnumerator5")
        (CallFunction|SetGameSpawned true))
      (:Is%20Not%20Valid
        (Development|PrintString "Error: Radar game-> Cant spawn BP_Render" true true "(R=1.000000,G=0.000000,B=0.000000,A=1.000000)" 5.0)))))

(event EventTogglePressed
  ;[1 1 1] Select event. Good or Bad point state switcher
  (if (Utilities|Enum|Equal(Enum) (Variables|Default|GetRadarState) "NewEnumerator5")
    (Variables|Default|SetPostColorCounter 0.0)
    (bind _ispointunderray (CallFunction|CheckPoint))
    (if _ispointunderray
      (if (Variables|Default|GetIsGoodPoint)
        (CallFunction|PlaySoundCue (Variables|Sounds|GetGoodPointSound) 0.0)
        (Variables|Default|SetRadarState "NewEnumerator3")
        (CallFunction|IncreaseComplete)
        (CallFunction|PlacePoint)
        (else
          (CallFunction|PlaySoundCue (Variables|Sounds|GetBadPointSound) 0.0 :!label _label)
          (Variables|Default|SetRadarState "NewEnumerator2")
          (CallFunction|DecreaseComplete)))
      (else
        (goto _label)))))

(fn SetRayFocus
  (params (RayDegree :type E_RadarFocus%20Enum :default "NewEnumerator0"))
  ;[1 1 1] Set Ray focus angle specified by game setting
  (switch Utilities|FlowControl|Switch|SwitchonE_RadarFocus RayDegree
    (:NewEnumerator0
      (LocalVariables|SetFocusMultiplier 24.0)
      (Variables|Default|SetRayFocusAngle 15.0))
    (:NewEnumerator1
      (LocalVariables|SetFocusMultiplier 12.0)
      (Variables|Default|SetRayFocusAngle 3e+01))
    (:NewEnumerator2
      (LocalVariables|SetFocusMultiplier 8.0)
      (Variables|Default|SetRayFocusAngle 45.0))
    (:NewEnumerator3
      (LocalVariables|SetFocusMultiplier 6.0)
      (Variables|Default|SetRayFocusAngle 6e+01)))
  (Rendering|Material|SetScalarParameterValue (Variables|Default|GetRadarRayMaterial) "FocusSize" (LocalVariables|GetFocusMultiplier) :!class /Script/Engine.MaterialInstanceDynamic))

(fn PlacePoint
  (bind _radarraymaterial (Variables|Default|GetRadarRayMaterial))
  ;[1 1 1] Place randomly Good or Bad point not under current Ray area
  (bind _output_get (Variables|Default|SetIsGoodPoint (<= (Math|Random|RandomIntegerinRange 0 9) 3)))
  (if _output_get
    (LocalVariables|SetTempPointColor (Variables|GameRadar|GetGoodPointColor))
    (else
      (LocalVariables|SetTempPointColor (Variables|GameRadar|GetBadPointColor))))
  (bind _output_get_2 (Variables|Default|SetPointLocation (Math|Vector|RotateVector (Math|Vector|MakeVector 0.0 0.0 (Math|Random|RandomFloatinRange (Variables|Default|GetMinPointRange) (Variables|Default|GetMaxPointRange))) (Math|Rotator|MakeRotator 0.0 (Math|Float|Clamp(Float) (+ (Math|Random|RandomFloatinRange 0.0 (/ (- 3.6e+02 (Variables|Default|GetRayFocusAngle)) 1.5)) (* (Variables|Default|GetRayCounter) 3.6e+02)) 0.0 3.6e+02) 0.0))))
  (Rendering|Material|SetScalarParameterValue _radarraymaterial "PointX" (+ (.X (Math|Vector|BreakVector _output_get_2)) 0.5) :!class /Script/Engine.MaterialInstanceDynamic)
  (Rendering|Material|SetScalarParameterValue _radarraymaterial "PointY" (+ (* (.Z (Math|Vector|BreakVector _output_get_2)) -1.0) 0.5) :!class /Script/Engine.MaterialInstanceDynamic)
  (Rendering|Material|SetVectorParameterValue _radarraymaterial "PointColor" (LocalVariables|GetTempPointColor) :!class /Script/Engine.MaterialInstanceDynamic)
  (Variables|Default|SetPointUnderRay false))

(fn CreateDynamicMaterial
  ;[1 1 1] Create Radar dynamic material
  (bind _returnvalue (Rendering|Material|CreateDynamicMaterialInstance "/Game/MiniGames/Materials/Radar/M_RadarRay.M_RadarRay" "None" "None" :!class /Script/Engine.KismetMaterialLibrary))
  (bind _output_get (Variables|Default|SetRadarRayMaterial _returnvalue))
  (return _output_get))

(fn RotateRay
  (params (DeltaTime :type Float%20%28single-precision%29))
  ;[1 1 1] Rotate Ray with defined speed
  (Rendering|Material|SetScalarParameterValue (Variables|Default|GetRadarRayMaterial) "RayAngle" (Variables|Default|GetRayCounter) :!class /Script/Engine.MaterialInstanceDynamic)
  (bind _output_get (Variables|Default|SetRayCounter (+ (Variables|Default|GetRayCounter) (* DeltaTime (Variables|GameRadar|GetRaySpeed)))))
  (if (>= _output_get 1.0)
    (Variables|Default|SetRayCounter (- _output_get 1.0))))

(fn CheckPoint
  (bind _pointlocation (Variables|Default|GetPointLocation))
  (bind (_x _y _z) (Math|Vector|BreakVector _pointlocation))
  (bind _returnvalue (Math|Float|Square _z))
  (bind _returnvalue_2 (Math|Float|Square _x))
  (bind _returnvalue_3 (+ _returnvalue_2 _returnvalue))
  (bind _returnvalue_4 (Math|Float|Sqrt _returnvalue_3))
  (bind _returnvalue_5 (/ _z _returnvalue_4))
  (bind _returnvalue_6 (Class|KismetMathLibrary|DegAcos _returnvalue_5))
  ;[1 1 1] Ceck if point is under ray or not. Return true if under ray
  (LocalVariables|SetOutResult false)
  (if (>= _x 0.0)
    (LocalVariables|SetTempPointAngle (- 3.6e+02 _returnvalue_6))
    (else
      (LocalVariables|SetTempPointAngle _returnvalue_6)))
  (LocalVariables|SetTestRayAngle (* (Variables|Default|GetRayCounter) 3.6e+02))
  (bind _output_get (LocalVariables|SetRayTwoAngle (- (LocalVariables|GetTestRayAngle) (Variables|Default|GetRayFocusAngle))))
  (if (and (< _output_get 0.0) (> (LocalVariables|GetTempPointAngle) 1.8e+02))
    (LocalVariables|SetRayTwoAngle (+ _output_get 3.6e+02))
    (if (> (LocalVariables|GetTempPointAngle) (LocalVariables|GetRayTwoAngle))
      (LocalVariables|SetOutResult true :!label _label))
    (elif (and (> (LocalVariables|GetTestRayAngle) (LocalVariables|GetTempPointAngle)) (> (LocalVariables|GetTempPointAngle) (LocalVariables|GetRayTwoAngle)))
      (goto _label)
      (else
        _)))
  (return (LocalVariables|GetOutResult)))

(fn SetPostColor
  (params (Color :type Linear%20Color%20Structure) (Counter :type Float%20%28single-precision%29))
  (bind _radarraymaterial (Variables|Default|GetRadarRayMaterial))
  ;[1 1 1] Pass post color and counter to material
  (Rendering|Material|SetScalarParameterValue _radarraymaterial "PostCounter" Counter :!class /Script/Engine.MaterialInstanceDynamic)
  (Rendering|Material|SetVectorParameterValue _radarraymaterial "PostColor" Color :!class /Script/Engine.MaterialInstanceDynamic))